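; Stage 3 Cyber Samurai enemy that extends a parent enemy class with melee montage attacks and a teleport strike.
; Finding a target triggers a high-damage opening Skill 3; later attacks randomly pick the normal attack or one of three skills.
; Montage callbacks toggle hit availability, and Skill 3 notifies spawn a burst effect and teleport it to the player.
; Hiton/HitOff events toggle weapon collision, and incoming damage goes to shared hit/death processing.
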(event `self.ReceiveBeginPlay`
  (`parent.ReceiveBeginPlay`)
  (`self.SetWeaponHit` (`self.WeaponHit`))
  (set `self.ChaseSpeed` 3000.0)
  (`self.SetCooltime` 2.0))

(event `/Game/Enemy/AI/BPI_PlayerTargeted.TargetFound`
  ; 전투 시작 스킬 사용
  (`GameplayStatics.PlaySoundAtLocation` "/Game/Assets/SoundEffects/Enemy/Stage2/SW_EnemySkeletonGuardBattleStart.SW_EnemySkeletonGuardBattleStart" (`self.K2_GetActorLocation`) (struct) 1.0 1.0 0.0 null null null null)
  (`self.StartSkill`))

(event `/Game/Enemy/AI/BPI_Enemy.Attack`
  (params (TargetActor :type "Actor Object Reference"))
  ; 공격 분배 : 기본 공격 / 스킬 1, 2, 3
  (switch `int` (`KismetMathLibrary.RandomIntegerInRange` 0 3)
    (:`0`
      (`self.NormalAttack`))
    (:`1`
      (`self.Skill1`))
    (:`2`
      (`self.Skill2`))
    (:`3`
      (`self.Skill3`))))

(event `/Game/Battle/BPI_HitDetect.HitOn`
  ; 공격 시 Collision On / Off
  (`PrimitiveComponent.SetCollisionEnabled` (`self.WeaponHit`) "QueryOnly"))

(event `/Game/Battle/BPI_HitDetect.HitOff`
  ; 공격 시 Collision On / Off
  (`PrimitiveComponent.SetCollisionEnabled` (`self.WeaponHit`) "NoCollision"))

(event `self.ReceiveAnyDamage`
  (params (Damage :type "Float (single-precision)") (DamageType :type "DamageType Object Reference") (InstigatedBy :type "Controller Object Reference") (DamageCauser :type "Actor Object Reference"))
  ; 받은 데미지 처리
  (`self.ProcessDamage` Damage (`self.HitMotionDamage`) "/Game/Enemy/Stage2/Animations/Move/AM_EnemySkeletonHit.AM_EnemySkeletonHit" (`self.Montage to Play`) (`self.Mesh`) "/Game/Enemy/Stage3/Animations/Move/AM_EnemyCyberSamuraiDeath.AM_EnemyCyberSamuraiDeath" (`self.BodyGuard`)))

(fn `SetCooltime`
  (params (Cooltime :type "Float (double-precision)"))
  (`parent.SetCooltime` Cooltime))

(fn `UserConstructionScript`
  (`parent.UserConstructionScript`))