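; Stage 2 skeleton pawn enemy with a montage-driven melee attack and an overhead-style HP widget.
; Attack sets damage and plays a montage whose notify opens a player hit window, alongside weapon collision toggled by Hiton/HitOff.
; Damage plays a hit montage and sound while a timeline lerps the health bar.
; At zero health it ragdolls with a death sound, then is destroyed after a delay.
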(event `self.ReceiveBeginPlay`
  (`parent.ReceiveBeginPlay`)
  ; 게임 시작 시 무기 충돌 Off. 이후 공격 시 On / Off 되도록 설정
  ; 무기 컴포넌트만 overlap 발생하도록 설정
  (`PrimitiveComponent.SetCollisionEnabled` (`self.WeaponHit`) "NoCollision")
  (add `PrimitiveComponent.OnComponentBeginOverlap` (`self.WeaponHit`) (delegate `WeaponOverlapped`))
  (bind (_output_get _outputpin) (`self.SetHPWidget`))
  (`/Game/Enemy/WBP_SkeletonPawnHP.UpdateHP` _output_get _outputpin _outputpin))

(event `WeaponOverlapped`
  (params (OverlappedComponent :type "PrimitiveComponent Object Reference") (OtherActor :type "Actor Object Reference") (OtherComp :type "PrimitiveComponent Object Reference") (OtherBodyIndex :type Integer) (bFromSweep :type Boolean) (SweepResult :type "HitResult Structure (by ref)"))
  ; 게임 시작 시 무기 충돌 Off. 이후 공격 시 On / Off 되도록 설정
  ; 무기 컴포넌트만 overlap 발생하도록 설정
  (`self.ApplyDamage` OtherActor (`self.Damage`)))

(event `/Game/Enemy/AI/BPI_Enemy.Attack`
  (params (TargetActor :type "Actor Object Reference"))
  ; 스켈레톤 병사 기본 공격
  (set `self.Damage` 5.0)
  (`self.HitDetect`))

(event `self.ReceiveActorBeginOverlap`
  (params (OtherActor :type "Actor Object Reference"))
  ; Hit 판정 시 데미지 적용
  (if (and (== OtherActor (`GameplayStatics.GetPlayerPawn` 0)) (`self.bHitAvailable`))
    (set `self.bHitAvailable` false)
    (`GameplayStatics.ApplyDamage` OtherActor (`self.Damage`) null self)))

(event `self.ReceiveAnyDamage`
  (params (Damage :type "Float (single-precision)") (DamageType :type "DamageType Object Reference") (InstigatedBy :type "Controller Object Reference") (DamageCauser :type "Actor Object Reference"))
  (bind _currenthealth (`self.CurrentHealth`))
  (bind _mesh (`self.Mesh`))
  ; HP
  (`self.PlayHit`)
  (set `self.StartHealth` _currenthealth)
  (set `self.TargetHealth` (`KismetMathLibrary.FClamp` (- _currenthealth Damage) 0.0 (`self.MaxHealth`)))
  (`GameplayStatics.PlaySoundAtLocation` "/Game/Assets/SoundEffects/Common/SW_Hit.SW_Hit" (`self.K2_GetActorLocation`) (struct) 1.0 1.0 0.0 null null null null)
  (bind (_direction _damagealpha) (`Timeline|타임라인` :!via `PlayFromStart`)
    (:`Update`
      (`/Game/Enemy/WBP_SkeletonPawnHP.UpdateHP` (`self.Target`) (`KismetMathLibrary.Lerp` (`self.StartHealth`) (`self.TargetHealth`) _damagealpha) (`self.MaxHealth`))
      (if (not (`self.bIsDead?`))
        (bind _output_get (set `self.CurrentHealth` (`self.TargetHealth`)))
        (if (<= _output_get 0.0)
          (set `self.bIsDead?` true)
          (`PrimitiveComponent.SetCollisionProfileName` _mesh (`self.In Collision Profile Name`) true)
          (`PrimitiveComponent.SetSimulatePhysics` _mesh true)
          (`GameplayStatics.PlaySoundAtLocation` "/Game/Assets/SoundEffects/Enemy/Stage2/SW_EnemySkeletonPawnDead.SW_EnemySkeletonPawnDead" (`self.K2_GetActorLocation`) (struct) 1.0 1.0 0.0 null null null null)
          (`PrimitiveComponent.SetCollisionEnabled` (`self.CapsuleComponent`) "NoCollision")
          (`KismetSystemLibrary.Delay` 2.5)
          (`self.K2_DestroyActor`))))))

(event `/Game/Battle/BPI_HitDetect.HitOn`
  ; 공격 시 Collision On / Off
  (`PrimitiveComponent.SetCollisionEnabled` (`self.WeaponHit`) "QueryOnly"))

(event `/Game/Battle/BPI_HitDetect.HitOff`
  ; 공격 시 Collision On / Off
  (`PrimitiveComponent.SetCollisionEnabled` (`self.WeaponHit`) "NoCollision"))

(fn `ApplyDamage`
  (params (TargetActor :type "Actor Object Reference") (InDamage :type "Float (double-precision)"))
  (`parent.ApplyDamage` TargetActor InDamage))

(fn `SetAttacking`
  (params (InIsAttacking :type Boolean :default false)))

(fn `UserConstructionScript`
  (`parent.UserConstructionScript`))