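; Base enemy Blueprint providing walk/chase speed, weapon damage, health and death logic, with montages and meshes passed in by callers.
; Weapon overlaps, bound with collision initially off, damage only the player pawn.
; ProcessDamage plays a hit reaction above a damage threshold, clamps health and broadcasts it through OnBossHPChanged.
; Death disables body collision, sets a Blackboard flag, broadcasts OnDead on montage notify and destroys the actor on completion.
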(event `self.ReceiveBeginPlay`
  (set `CharacterMovementComponent.MaxWalkSpeed` (`self.WalkSpeed`) (`self.CharacterMovement`))
  (bind _output_get (set `self.CurrentHealth` (`self.MaxHealth`)))
  (`self.OnBossHPChanged` _output_get _output_get))

(event `/Game/Enemy/AI/BPI_PlayerTargeted.SetChaseSpeed`
  (set `CharacterMovementComponent.MaxWalkSpeed` (`self.ChaseSpeed`) (`self.CharacterMovement`)))

(event `SetWeaponHit`
  (params (InWeaponHit :type "PrimitiveComponent Object Reference"))
  ; 게임 시작 시 무기 충돌 Off. 이후 공격 시 On / Off 되도록 설정
  ; 무기 컴포넌트만 overlap 발생하도록 설정
  (`PrimitiveComponent.SetCollisionEnabled` InWeaponHit "NoCollision")
  (add `PrimitiveComponent.OnComponentBeginOverlap` InWeaponHit (delegate `WeaponOverlapped`)))

(event `WeaponOverlapped`
  (params (OverlappedComponent :type "PrimitiveComponent Object Reference") (OtherActor :type "Actor Object Reference") (OtherComp :type "PrimitiveComponent Object Reference") (OtherBodyIndex :type Integer) (bFromSweep :type Boolean) (SweepResult :type "HitResult Structure (by ref)"))
  ; 게임 시작 시 무기 충돌 Off. 이후 공격 시 On / Off 되도록 설정
  ; 무기 컴포넌트만 overlap 발생하도록 설정
  (`self.ApplyDamage` OtherActor (`self.Damage`)))

(event `ProcessDamage`
  (params (Damage :type "Float (double-precision)") (HitMotionDamage :type "Float (double-precision)") (HitMotionMontage :type "AnimMontage Object Reference") (CurrentMontage :type "AnimMontage Object Reference") (Mesh :type "SkeletalMeshComponent Object Reference") (DeadMontage :type "AnimMontage Object Reference") (BodyGuard :type "CapsuleComponent Object Reference"))
  ; 받은 데미지 처리
  (if (not (`self.bIsDead`))
    (`self.PlayHit` Damage HitMotionDamage HitMotionMontage CurrentMontage Mesh)
    (bind _currenthealth (`self.CalculateHP` Damage))
    (bind _output_get (set `self.CurrentHealth` _currenthealth))
    (`self.OnBossHPChanged` self _output_get (`self.MaxHealth`))
    (if (<= (`self.CurrentHealth`) 0.0)
      (`PrimitiveComponent.SetCollisionEnabled` BodyGuard "NoCollision")
      (`PrimitiveComponent.SetCollisionEnabled` (`self.CapsuleComponent`) "NoCollision")
      (`self.PlayDead` CurrentMontage Mesh DeadMontage))))

(fn `ApplyDamage`
  (params (TargetActor :type "Actor Object Reference") (InDamage :type "Float (double-precision)"))
  (if (== (`GameplayStatics.GetPlayerPawn` 0) TargetActor)
    (`GameplayStatics.ApplyDamage` TargetActor InDamage)))

(fn `SetAttacking`
  (params (InIsAttacking :type Boolean))
  (locals (IsAttacking :type Name :default "IsAttacking"))
  (bind _returnvalue (`AIBlueprintHelperLibrary.GetBlackboard` (`self.GetController`)))
  (`/Engine/EditorBlueprintResources/StandardMacros.IsValid` _returnvalue
    (:`Is Valid`
      (`BlackboardComponent.SetValueAsBool` _returnvalue (`local.IsAttacking`) InIsAttacking))))

(fn `UserConstructionScript`)